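; BP_Item is a randomized pickup that grants ThirdPersonCharacter a coin, power-up or life.
; The construction script rolls ItemType through cascading random checks, heavily favoring coins, and sets a matching food or condiment mesh.
; On a StaticMesh hit by that character, it calls the type's pickup and any paired reset (speed, double coin, invincibility), then destroys itself.
; Coins (fries) count twice while IsDouble is active and play a sound.
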(event OnComponentHit(StaticMesh)
  (params (HitComponent :type Primitive%20Component%20Object%20Reference) (OtherActor :type Actor%20Object%20Reference) (OtherComp :type Primitive%20Component%20Object%20Reference) (NormalImpulse :type Vector :default "0, 0, 0") (Hit :type Hit%20Result%20Structure%20%28by%20ref%29))
  (bind _asthird_person_character (Utilities|Casting|CastToThirdPersonCharacter OtherActor))
  (switch int (Variables|Default|GetItemType)
    (:Default
      (Default|AddCoin _asthird_person_character :!label _label)
      (if (Variables|/Game/Blueprints/ThirdPersonCharacter.ThirdPersonCharacter_C|GetisDouble _asthird_person_character)
        (Default|AddCoin _asthird_person_character))
      (Audio|PlaySoundatLocation 0 (Transformation|GetActorLocation)))
    (:0
      (goto _label))
    (:1
      (Default|PickupKetchup _asthird_person_character)
      (Default|ResetSpeed _asthird_person_character :!label _label_2))
    (:2
      (Default|PickupJam _asthird_person_character)
      (goto _label_2))
    (:3
      (Default|PickupdoubleCoin _asthird_person_character)
      (Default|ResetDouble _asthird_person_character))
    (:4
      (Default|PickupMayo _asthird_person_character)
      (Default|ResetInvincible _asthird_person_character))
    (:5
      (Default|PickupLife _asthird_person_character)))
  (Actor|DestroyActor))

(event EventBeginPlay)

(event Collision|EventActorBeginOverlap
  (params (OtherActor :type Actor%20Object%20Reference)))

(event EventTick
  (params (DeltaSeconds :type Float%20%28single-precision%29)))

(fn ConstructionScript
  (bind _staticmesh (Variables|Default|GetStaticMesh))
  (CallFunction|GetRandomType)
  (switch int (Variables|Default|GetItemType)
    (:Default
      (Components|StaticMesh|SetStaticMesh _staticmesh "/Game/Geometry/Meshes/Fries_001.Fries_001" :!label _label))
    (:0
      (goto _label))
    (:1
      (Components|StaticMesh|SetStaticMesh _staticmesh "/Game/Geometry/Meshes/Ketchup_bottle.Ketchup_bottle"))
    (:2
      (Components|StaticMesh|SetStaticMesh _staticmesh "/Game/Geometry/Meshes/Jelly_Jar.Jelly_Jar"))
    (:3
      (Components|StaticMesh|SetStaticMesh _staticmesh "/Game/Geometry/Meshes/Pepper_Shaker.Pepper_Shaker"))
    (:4
      (Components|StaticMesh|SetStaticMesh _staticmesh "/Game/Geometry/Meshes/Mayo_Jar.Mayo_Jar"))
    (:5
      (Components|StaticMesh|SetStaticMesh _staticmesh "/Game/Geometry/Meshes/Salt_Shaker.Salt_Shaker"))))

(fn GetRandomType
  (bind _returnvalue (Math|Random|RandomIntegerinRange 0 100))
  (if (< _returnvalue 80)
    (Variables|Default|SetItemType 0)
    (elif (< _returnvalue 85)
      (Variables|Default|SetItemType 1)
      (elif (< _returnvalue 90)
        (Variables|Default|SetItemType 2)
        (elif (< _returnvalue 95)
          (Variables|Default|SetItemType 3)
          (elif (< _returnvalue 98)
            (Variables|Default|SetItemType 4)
            (else
              (Variables|Default|SetItemType 5))))))))