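; Map segment Blueprint, apparently the starting piece, that exposes an AttachPoint world transform, likely for chaining the next segment.
; Its construction script randomly spawns either one blocker or four items as child actor components.
; Blockers land at random points inside the HazardArea box and items inside the ItemArea box, using each box's relative location and extent.
; The event graph holds only disabled placeholder events.
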(event EventBeginPlay)

(event Collision|EventActorBeginOverlap
  (params (OtherActor :type Actor%20Object%20Reference)))

(event EventTick
  (params (DeltaSeconds :type Float%20%28single-precision%29)))

(fn ConstructionScript
  (switch int (Math|Random|RandomIntegerinRange 0 1)
    (:0
      (CallFunction|SpawnBlocker))
    (:1
      (CallFunction|SpawnItem)
      (CallFunction|SpawnItem)
      (CallFunction|SpawnItem)
      (CallFunction|SpawnItem))))

(fn GetAttachTransform
  (return (Transformation|GetWorldTransform (Variables|Default|GetattachPoint))))

(fn SpawnBlocker
  (bind _hazardarea (Variables|Default|GethazardArea))
  (AddComponent|AddChildActorComponent false (Math|Conversions|ToTransform(Vector) (Math|Random|RandomPointinBoundingBox (Variables|/Script/Engine.SceneComponent|GetRelativeLocation _hazardarea) (Variables|/Script/Engine.BoxComponent|GetBoxExtent _hazardarea)))))

(fn SpawnItem
  (bind _itemarea (Variables|Default|GetitemArea))
  (AddComponent|AddChildActorComponent false (Math|Conversions|ToTransform(Vector) (Math|Random|RandomPointinBoundingBox (Variables|/Script/Engine.SceneComponent|GetRelativeLocation _itemarea) (Variables|/Script/Engine.BoxComponent|GetBoxExtent _itemarea)))))