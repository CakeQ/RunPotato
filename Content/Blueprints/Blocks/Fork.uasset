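; Fork is a hazard Blueprint that damages the player character on contact.
; When its static mesh begins overlapping a ThirdPersonCharacter that is not invincible, it removes one life, plays a hurt sound and calls the character's Death when lives reach zero.
; The fork destroys itself after any overlap with that character, even if the character is invincible.
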(event OnComponentBeginOverlap(StaticMesh)
  (params (OverlappedComponent :type Primitive%20Component%20Object%20Reference) (OtherActor :type Actor%20Object%20Reference) (OtherComp :type Primitive%20Component%20Object%20Reference) (OtherBodyIndex :type Integer) (bFromSweep :type Boolean) (SweepResult :type Hit%20Result%20Structure%20%28by%20ref%29))
  (bind _asthird_person_character (Utilities|Casting|CastToThirdPersonCharacter OtherActor))
  (if (Variables|/Game/Blueprints/ThirdPersonCharacter.ThirdPersonCharacter_C|GetisInvincible _asthird_person_character)
    _
    (else
      (bind _output_get (Variables|/Game/Blueprints/ThirdPersonCharacter.ThirdPersonCharacter_C|SetLives _asthird_person_character (- (Variables|/Game/Blueprints/ThirdPersonCharacter.ThirdPersonCharacter_C|GetLives _asthird_person_character) 1)))
      (Audio|PlaySound2D "/Game/Audio/hurt.hurt")
      (if (== _output_get 0)
        (Default|Death _asthird_person_character))))
  (Actor|DestroyActor))

(event EventBeginPlay)

(event Collision|EventActorBeginOverlap
  (params (OtherActor :type Actor%20Object%20Reference)))

(event EventTick
  (params (DeltaSeconds :type Float%20%28single-precision%29)))

(fn ConstructionScript)